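; BP_Array is a data-structures Blueprint that demonstrates queue and stack operations on a single shared array.
; Enqueue and Push both append to the end, Dequeue removes the first element, and Pop removes the last, each printing the value to screen.
; PrintArray prints every element.
; Pop returns DequeueData instead of the PopData it removes, and neither removal function has a return path for an empty array.
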(event EventEnqueue
  (params (Data :type Integer))
  (Utilities|Array|Add (Variables|Default|GetArray) Data)
  (Development|PrintString 0 (Utilities|String|Append "Queued: " (Utilities|String|ToString(Integer) Data)) true true "(R=0.000000,G=0.660000,B=1.000000,A=1.000000)" 2.0 "1"))

(event EventPush
  (params (Data :type Integer))
  (Utilities|Array|Add (Variables|Default|GetArray) Data)
  (Development|PrintString 0 (Utilities|String|Append "Pushed: " (Utilities|String|ToString(Integer) Data)) true true "(R=0.000000,G=0.660000,B=1.000000,A=1.000000)" 2.0 "1"))

(fn PrintArray
  (for _array_element (Variables|Default|GetArray)
    (Development|PrintString 0 (Utilities|String|ToString(Integer) _array_element)))
  (return))

(fn Dequeue
  (bind _array (Variables|Default|GetArray))
  (if (Utilities|Array|IsNotEmpty _array)
    (Variables|Default|SetDequeueData (Utilities|Array|Get(acopy) _array))
    (Utilities|Array|RemoveIndex (Variables|Default|GetArray))
    (Development|PrintString 0 (Utilities|String|Append "Dequeued: " (Utilities|String|ToString(Integer) (Variables|Default|GetDequeueData))))
    (return (Variables|Default|GetDequeueData))))

(fn Pop
  (bind _array (Variables|Default|GetArray))
  (bind _returnvalue (Utilities|Array|LastIndex _array))
  (if (Utilities|Array|IsNotEmpty _array)
    (Variables|Default|SetPopLastIndex _returnvalue)
    (Variables|Default|SetPopData (Utilities|Array|Get(acopy) _array _returnvalue))
    (Utilities|Array|RemoveIndex (Variables|Default|GetArray) (Variables|Default|GetPopLastIndex))
    (Development|PrintString 0 (Utilities|String|Append "Poped: " (Utilities|String|ToString(Integer) (Variables|Default|GetPopData))))
    (return (Variables|Default|GetDequeueData))))